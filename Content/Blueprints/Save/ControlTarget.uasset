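; ControlTarget is a one-time checkpoint actor that records player progress for the current level.
; When anything begins overlapping its Sphere, it checks for a save slot named after the level and does nothing if one exists.
; Otherwise it creates a Save object, passes it its own location, the level name, and the player Bun's HP and jump count, then destroys itself.
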(event `self.Sphere.OnComponentBeginOverlap`
  (params (OverlappedComponent :type "PrimitiveComponent Object Reference") (OtherActor :type "Actor Object Reference") (OtherComp :type "PrimitiveComponent Object Reference") (OtherBodyIndex :type Integer) (bFromSweep :type Boolean) (SweepResult :type "HitResult Structure (by ref)"))
  (bind _returnvalue (`GameplayStatics.GetCurrentLevelName` true))
  (bind _returnvalue_2 (`GameplayStatics.DoesSaveGameExist` _returnvalue))
  (if (not _returnvalue_2)
    (bind _returnvalue_3 (`GameplayStatics.CreateSaveGameObject` "/Game/Blueprints/Save/Save.Save_C"))
    (set `self.SaveGame` _returnvalue_3)
    (bind (_hp _count_jump) (`self.BunProperties`))
    (`/Game/Blueprints/Save/Save.Save` (`self.SaveGame`) (`self.K2_GetActorLocation`) _returnvalue _hp _count_jump)
    (`self.K2_DestroyActor`)))

(fn `BunProperties`
  (returns (HP :type "Float (double-precision)") (`Count Jump` :type "Float (double-precision)"))
  (bind _asbun (cast `/Game/Blueprints/Character/Bun` (`GameplayStatics.GetPlayerPawn` 0)))
  (return (`FallAndContinueCharacter.HP` _asbun) (`FallAndContinueCharacter.GeneralCountJump` _asbun)))

(fn `UserConstructionScript`)