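; Save game object that stores player progress and game settings and writes itself to save slots.
; Save copies position, HP and jump count into its variables, then saves to the slot name passed in.
; SaveSettings does the same for resolution and graphics, using a fixed "Settings" slot.
; DeleteGame removes a slot by name, and all slot operations use user index 0.
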(fn `DeleteGame`
  (params (NameSlot :type String))
  (`GameplayStatics.DeleteGameInSlot` NameSlot))

(fn `Save`
  (params (Position :type "Vector Structure") (String :type String) (HP :type "Float (double-precision)") (CountJump :type "Float (double-precision)"))
  (set `self.Position` Position)
  (set `self.HP` HP)
  (set `self.CountJump` CountJump)
  (`GameplayStatics.SaveGameToSlot` self String))

(fn `SaveSettings`
  (params (Resolution :type Integer) (Graphics :type "Array of Integer"))
  (set `self.resolution` Resolution)
  (set `self.Graphics` Graphics)
  (`GameplayStatics.SaveGameToSlot` self "Settings"))