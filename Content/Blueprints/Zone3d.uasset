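; Zone3d is a box trigger zone for a side-scroller that, judging by its name, marks a switch to a 3D view.
; On any actor overlap it casts player pawn 0 to 2DSideScrollerCharacter, without checking which actor entered.
; It then toggles that character's Camera active state and snaps its Sprite to a fixed world rotation.
; The construction script sizes the Box from the Size variable.
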(event `self.ReceiveActorBeginOverlap`
  (params (OtherActor :type "Actor Object Reference"))
  (bind _as2dside_scroller_character (cast `/Game/Blueprints/Character/2DSideScrollerCharacter` (`GameplayStatics.GetPlayerPawn` 0)))
  (bind _output_get (set `self.Bun` _as2dside_scroller_character))
  (`ActorComponent.ToggleActive` (`/Game/Blueprints/Character/2DSideScrollerCharacter.Camera` _output_get))
  (`SceneComponent.K2_SetWorldRotation` (`PaperCharacter.Sprite` _output_get) (struct :`Yaw` 100.0) false false))

(fn `UserConstructionScript`
  (`BoxComponent.SetBoxExtent` (`self.Box`) (`self.size`) true))