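; RabbitKiller is a 2D flipbook enemy that hops at the nearby player, damages it on hit, and triggers the WIN widget on death.
; Tick drives timed impulse hops, facing and sleep, angry or death animations.
; Tick also recreates the health-bar widget every frame, setting its material progress from Hp.
; At zero Hp, Tick spawns PlusHP at world origin every frame until the delayed destroy.
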(event `self.ReceiveTick`
  (params (DeltaSeconds :type "Float (single-precision)"))
  (bind _returnvalue (`GameplayStatics.GetPlayerPawn` 0))
  (bind _flipbook (`self.flipbook`))
  (bind _returnvalue_2 (> (.x (`self.K2_GetActorLocation` _returnvalue)) (.x (`self.K2_GetActorLocation`))))
  (set `self.dt` DeltaSeconds)
  (set `self.pd` (`self.GetDistanceTo` _returnvalue))
  (`self.WB`)
  (`|ExecutionSequence`
    (:`then_0`
      (if (<= (`self.reset_tmr`) 0.0)
        (if (<= (`self.pd`) 800.0)
          (set `self.reset_tmr` (`self.reset`)))
        (else
          (set `self.reset_tmr` (- (`self.reset_tmr`) (`self.dt`))))))
    (:`then_1`
      (if (and (<= (`self.pd`) 800.0) (== (`self.reset_tmr`) (`self.reset`)))
        (if _returnvalue_2
          (set `self.xk` 1.0)
          (else
            (set `self.xk` -1.0)))
        (`PrimitiveComponent.AddImpulse` (`self.collis_sph`) (`KismetMathLibrary.MakeVector` (* (`self.spd_x`) (`self.xk`)) 0.0 (`self.spd_z`)) "None" true)))
    (:`then_2`
      (`|ExecutionSequence`
        (:`then_0`
          (if _returnvalue_2
            (`SceneComponent.K2_SetWorldRotation` _flipbook (struct :`Yaw` 180.0) false false)
            (else
              (`SceneComponent.K2_SetWorldRotation` :`self` _flipbook))))
        (:`then_1`
          (if (> (`KismetMathLibrary.VSize` (`self.GetVelocity`)) 0.0)
            (set `self.fb_anim` "/Game/sprite/Rabbit/AngryRabbit.AngryRabbit")
            (else
              (set `self.fb_anim` "/Game/sprite/Rabbit/SleepRabbit.SleepRabbit"))))
        (:`then_2`
          (if (<= (`self.hp`) 0.0)
            (set `self.fb_anim` "/Game/sprite/Rabbit/RabbitAngryDeath.RabbitAngryDeath")
            (`|SpawnActorFromClass` "/Game/Blueprints/PlusHP.PlusHP_C" (`KismetMathLibrary.MakeTransform` (0.0 0.0 0.0)) "AdjustIfPossibleButAlwaysSpawn" "OverrideRootScale" null null)))
        (:`then_3`
          (`PaperFlipbookComponent.SetFlipbook` (`self.flipbook`) (`self.fb_anim`)))))))

(event `WB`
  (bind _returnvalue (`|CreateWidget` "/Game/Blueprints/Widgets/HpForEnemy.HpForEnemy_C"))
  (bind _output_get (set `self.NewVar_0` _returnvalue))
  (`WidgetComponent.SetWidget` (`self.Widget`) _returnvalue)
  (bind _returnvalue_2 (`Image.GetDynamicMaterial` (`/Game/Blueprints/Widgets/HpForEnemy.Image_7` _output_get)))
  (`MaterialInstanceDynamic.SetScalarParameterValue` _returnvalue_2 "Progress" (/ (`self.hp`) 50.0)))

(event `self.ReceiveHit`
  (params (MyComp :type "PrimitiveComponent Object Reference") (Other :type "Actor Object Reference") (OtherComp :type "PrimitiveComponent Object Reference") (bSelfMoved :type Boolean) (HitLocation :type "Vector Structure") (HitNormal :type "Vector Structure") (NormalImpulse :type "Vector Structure") (Hit :type "HitResult Structure (by ref)"))
  (if (and (`self.ActorHasTag` Other "player") (> (`self.hp`) 0.0))
    (`GameplayStatics.ApplyDamage` Other (`self.dmg`))))

(event `self.ReceiveAnyDamage`
  (params (Damage :type "Float (single-precision)") (DamageType :type "DamageType Object Reference") (InstigatedBy :type "Controller Object Reference") (DamageCauser :type "Actor Object Reference"))
  (bind _output_get (set `self.hp` (- (`self.hp`) Damage)))
  (if (<= _output_get 0.0)
    (`KismetSystemLibrary.Delay` 0.6)
    (`self.K2_DestroyActor`)
    (bind _returnvalue (`|CreateWidget` "/Game/Blueprints/Widgets/WIN.WIN_C"))
    (`UserWidget.AddToViewport` _returnvalue 0)))

(fn `UserConstructionScript`)