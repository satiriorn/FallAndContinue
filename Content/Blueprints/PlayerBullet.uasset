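; PlayerBullet is a player projectile that deals impact and area damage when it hits, then destroys itself.
; On Hit, it copies its radial-effect setting to a struck BP_DENT_MASTER, then applies both full radial damage and point damage.
; It also adds a radial impulse to its own Sphere component and spawns an explosion emitter and attenuated boom sound at the impact point.
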(event `self.ReceiveHit`
  (params (MyComp :type "PrimitiveComponent Object Reference") (Other :type "Actor Object Reference") (OtherComp :type "PrimitiveComponent Object Reference") (bSelfMoved :type Boolean) (HitLocation :type "Vector Structure") (HitNormal :type "Vector Structure") (NormalImpulse :type "Vector Structure") (Hit :type "HitResult Structure (by ref)"))
  (bind (_bblockinghit _binitialoverlap _time _distance _location _impactpoint _normal _impactnormal _physmat _hitactor) (`GameplayStatics.BreakHitResult` Hit))
  (bind _returnvalue (`ActorComponent.GetOwner` (`self.ProjectileMovement`)))
  ;[0.2706 0.2706 0.2706] Radial Damage
  (bind _asbp_dent_master (cast `/Game/DENT/BluePrints/Destructibles/Destructibles_Master/BP_DENT_MASTER` _hitactor)
    (:`then`
      (set `/Game/DENT/BluePrints/Destructibles/Destructibles_Master/BP_DENT_MASTER.IsDamageRadial` (`self.DMRadialEffect`) _asbp_dent_master))
    (:`CastFailed`
      _))
  (`GameplayStatics.ApplyRadialDamage` :`BaseDamage` (`self.Damage`) :`Origin` _impactpoint :`DamageRadius` (`self.Radius`) :`DamageTypeClass` "/Script/Engine.DamageType" :`DamageCauser` _returnvalue :`InstigatedByController` null :`bDoFullDamage` true)
  (`GameplayStatics.ApplyPointDamage` _hitactor (`self.Damage`) _impactpoint Hit null _returnvalue)
  (`PrimitiveComponent.AddRadialImpulse` (`self.Sphere`) _impactpoint (`self.Radius`) (`self.Strenth`) "RIF_Constant" false)
  (`GameplayStatics.SpawnEmitterAtLocation` "/Game/DENT/Particles/P_Radial.P_Radial" _impactpoint)
  (`GameplayStatics.PlaySoundAtLocation` "/Game/DENT/Audio/S_Boom.S_Boom" _impactpoint (struct) 1.0 1.0 0.0 "/Game/DENT/Audio/Distance.Distance" null null) ; Play firing sound
  (`self.K2_DestroyActor`))

(fn `UserConstructionScript`)