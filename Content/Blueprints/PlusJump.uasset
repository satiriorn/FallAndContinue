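; PlusJump is a pickup actor that grants an extra jump when something overlaps its Box.
; On BeginPlay it casts and stores the game instance as MyGameInstance.
; An overlap increments the instance's CountJump while it is below three, and the actor destroys itself either way.
; The overlapping actor is not checked, so any overlap consumes the pickup.
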(event `self.ReceiveBeginPlay`
  (bind _asmy_game_instance (cast `/Game/Blueprints/MyGameInstance` (`GameplayStatics.GetGameInstance`)))
  (set `self.GI` _asmy_game_instance))

(event `self.Box.OnComponentBeginOverlap`
  (params (OverlappedComponent :type "PrimitiveComponent Object Reference") (OtherActor :type "Actor Object Reference") (OtherComp :type "PrimitiveComponent Object Reference") (OtherBodyIndex :type Integer) (bFromSweep :type Boolean) (SweepResult :type "HitResult Structure (by ref)"))
  (bind _gi (`self.GI`))
  (bind _countjump (`/Game/Blueprints/MyGameInstance.CountJump` _gi))
  (if (< _countjump 3.0)
    (bind _result (`/Engine/EditorBlueprintResources/StandardMacros.IncrementFloat` _countjump)
      (:`  `
        (set `/Game/Blueprints/MyGameInstance.CountJump` _result _gi)
        (`self.K2_DestroyActor`)))
    (else
      (`self.K2_DestroyActor`))))

(fn `UserConstructionScript`)