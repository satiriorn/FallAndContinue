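; Lift actor that moves its SpaceShip component between its origin and EndLocation, with travel time setting the timeline play rate.
; LiftForward and LiftBackward start the timeline, which lerps the relative location and flips direction after StopDelay at each end.
; Overlapping SafetyCollider during movement reverses the lift's direction.
; The construction script previews either endpoint through TestEndLocation.
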(event `self.ReceiveBeginPlay`
  (`TimelineComponent.SetPlayRate` (`self.LiftTimeline`) (/ 1.0 (`self.TravelTimeInSeconds`)))
  (set `self.TestEndLocation` true))

(event `self.SafetyCollider.OnComponentBeginOverlap`
  (params (OverlappedComponent :type "PrimitiveComponent Object Reference") (OtherActor :type "Actor Object Reference") (OtherComp :type "PrimitiveComponent Object Reference") (OtherBodyIndex :type Integer) (bFromSweep :type Boolean) (SweepResult :type "HitResult Structure (by ref)"))
  (bind _lifttimeline (`self.LiftTimeline`))
  (if (`ActorComponent.IsActive` _lifttimeline)
    (if (`TimelineComponent.IsReversing` _lifttimeline)
      (bind (_direction _lerp_alpha) (`Timeline|LiftTimeline` :!label _label)
        (:`Update`
          (`SceneComponent.K2_SetRelativeLocation` (`self.SpaceShip`) (`KismetMathLibrary.VLerp` (0.0 0.0 0.0) (`self.EndLocation`) _lerp_alpha) false false))
        (:`Finished`
          (`KismetSystemLibrary.Delay` (`self.StopDelay`))
          (switch `ETimelineDirection` _direction
            (:`Forward`
              (`self.LiftBackward`))
            (:`Backward`
              (`self.LiftForward`)))))
      (else
        (goto _label :!via `Reverse`)))))

(event `LiftForward`
  (goto _label :!via `PlayFromStart`))

(event `LiftBackward`
  (goto _label :!via `ReverseFromEnd`))

(fn `UserConstructionScript`
  (`SceneComponent.K2_SetRelativeLocation` (`self.SpaceShip`) (`KismetMathLibrary.SelectVector` (`self.EndLocation`) (0.0 0.0 0.0) (`self.TestEndLocation`)) false false))