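; PlusHP is a health pickup Blueprint for the Bun player pawn.
; BeginPlay caches the player pawn as Bun, and any overlap on its Sphere acts on that reference without checking the overlapping actor.
; Below full health, it adds a fixed amount when the deficit is large enough, otherwise adds the negative deficit, which lowers HP, then destroys itself.
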(event `self.ReceiveBeginPlay`
  (bind _asbun (cast `/Game/Blueprints/Character/Bun` (`GameplayStatics.GetPlayerPawn` 0)))
  (set `self.Bun` _asbun))

(event `self.Sphere.OnComponentBeginOverlap`
  (params (OverlappedComponent :type "PrimitiveComponent Object Reference") (OtherActor :type "Actor Object Reference") (OtherComp :type "PrimitiveComponent Object Reference") (OtherBodyIndex :type Integer) (bFromSweep :type Boolean) (SweepResult :type "HitResult Structure (by ref)"))
  (bind _bun (`self.Bun`))
  (bind _bun_2 (`self.Bun`))
  (bind _hp (`FallAndContinueCharacter.HP` (`self.Bun`)))
  (if (< _hp 100.0)
    (bind _output_get (set `self.HpPlus` (- _hp 100.0)))
    (if (<= _output_get -20.0)
      (set `FallAndContinueCharacter.HP` (+ (`FallAndContinueCharacter.HP` _bun_2) 20.0) _bun_2)
      (`self.K2_DestroyActor`)
      (else
        (set `FallAndContinueCharacter.HP` (+ (`FallAndContinueCharacter.HP` _bun) (`self.HpPlus`)) _bun)
        (`self.K2_DestroyActor`)))))

(fn `UserConstructionScript`)